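; BP_Ambulance is a clickable ambulance actor that opens a WBP_AmbulancePopOut option menu at the mouse position.
; On BeginPlay it creates the widget and binds its events for getting in or out, leaving and calling by radio.
; Those handlers delegate to BP_FPPlayerController, which sets the player's state, and a successful get-in notifies the widget.
; A shown flag prevents reopening the popup until selecting an option removes it.
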(event OnClicked(AmboMesh)
  (params (TouchedComponent :type Primitive%20Component%20Object%20Reference) (ButtonPressed :type Key%20Structure))
  (if (not (Variables|Default|GetWidgetShowed))
    (if (Utilities|IsValid (Variables|Default|GetWidgetPopUp))
      (CallFunction|AddWidget))))

(event Custom|AddWidget
  (bind _returnvalue (Game|GetPlayerController 0))
  (bind _widgetpopup (Variables|Default|GetWidgetPopUp))
  (bind (_locationx _locationy) (Game|Player|GetMousePosition _returnvalue))
  (Class|UserWidget|SetPositioninViewport _widgetpopup (Math|Vector2D|MakeVector2D _locationx _locationy) true)
  (UserInterface|Viewport|AddtoViewport _widgetpopup 0)
  (Variables|Default|SetWidgetShowed true))

(event Custom|GetInCar
  (bind _playercontroller (Variables|Default|GetPlayerController))
  (bind _returnvalue (Class|FPPlayerController|GetinAmbulance _playercontroller))
  (if _returnvalue
    (Class|FPPlayerController|SetDriveAmbulance _playercontroller)
    (Default|GetinSuc (Variables|Default|GetWidgetPopUp))))

(event Custom|LeaveAmbulance
  (bind _playercontroller (Variables|Default|GetPlayerController))
  (Class|FPPlayerController|GetOutAmbulance _playercontroller)
  (Class|FPPlayerController|SetNone _playercontroller)
  (Class|FPPlayerController|EnableOperations _playercontroller true))

(event Custom|Radio
  (Class|FPPlayerController|SetRadio (Variables|Default|GetPlayerController)))

(event Custom|RemoveWidget
  (Widget|RemovefromParent (Variables|Default|GetWidgetPopUp))
  (Variables|Default|SetWidgetShowed false))

(event Custom|GetOutAmbulance
  (bind _returnvalue (Class|FPPlayerController|SetGetOutAmbulance (Variables|Default|GetPlayerController)))
  (if _returnvalue
    _))

(event EventBeginPlay
  (bind _asbp_fpplayer_controller (Utilities|Casting|CastToBP_FPPlayerController (Game|GetPlayerController 0)))
  (Variables|Default|SetPlayerController _asbp_fpplayer_controller)
  (bind _returnvalue (UserInterface|CreateWidget "/Game/BPs/Widgets/WBP_AmbulancePopOut.WBP_AmbulancePopOut_C"))
  (bind _output_get (Variables|Default|SetWidgetPopUp _returnvalue))
  (EventDispatchers|BindEventtoOptionSelected _output_get (delegate Custom|RemoveWidget))
  (EventDispatchers|BindEventtoGetinAmbulanceEvent _output_get (delegate Custom|GetInCar))
  (EventDispatchers|BindEventtoLeaveAmbulanceEvent _output_get (delegate Custom|LeaveAmbulance))
  (EventDispatchers|BindEventtoCallAmbulanceEvent _output_get (delegate Custom|Radio))
  (EventDispatchers|BindEventtoGetOutAmbulanceEvent _output_get (delegate Custom|GetOutAmbulance)))

(fn ConstructionScript
  (Variables|Default|SetambulanceMesh (Variables|Default|GetAmboMesh)))