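; BP_ExFire is an extinguishable fire with clickable Fire and Smoke components, cleared in two stages.
; Clicks on either component share one handler, which acts only when the FPPlayerController's current operation is ExtinguishFire.
; While IsFire is set, a click destroys the Fire component and switches the state flags to smoke; otherwise it destroys the Smoke component.
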(event OnClicked(Fire)
  (params (TouchedComponent :type Primitive%20Component%20Object%20Reference) (ButtonPressed :type Key%20Structure))
  (bind _asfpplayer_controller (Utilities|Casting|CastToFPPlayerController (Game|GetPlayerController 0)))
  (bind _returnvalue (Class|FPPlayerController|GetCurrentOperation _asfpplayer_controller))
  (if (Utilities|Enum|Equal(Enum) _returnvalue "ExtinguishFire")
    (if (Variables|Default|Getis_Fire)
      (Components|DestroyComponent (Variables|Default|GetFire))
      (Variables|Default|Setis_Fire false)
      (Variables|Default|Setis_Smoke true)
      (else
        (Components|DestroyComponent (Variables|Default|GetSmoke))))))

(event OnClicked(Smoke)
  (params (TouchedComponent :type Primitive%20Component%20Object%20Reference) (ButtonPressed :type Key%20Structure))
  (bind _asfpplayer_controller (Utilities|Casting|CastToFPPlayerController (Game|GetPlayerController 0)))
  (bind _returnvalue (Class|FPPlayerController|GetCurrentOperation _asfpplayer_controller))
  (if (Utilities|Enum|Equal(Enum) _returnvalue "ExtinguishFire")
    (if (Variables|Default|Getis_Fire)
      (Components|DestroyComponent (Variables|Default|GetFire))
      (Variables|Default|Setis_Fire false)
      (Variables|Default|Setis_Smoke true)
      (else
        (Components|DestroyComponent (Variables|Default|GetSmoke))))))

(fn ConstructionScript)