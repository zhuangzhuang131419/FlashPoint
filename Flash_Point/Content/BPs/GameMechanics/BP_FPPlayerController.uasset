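; Player controller for the Flash Point firefighting game, handling player name, role widget classes and cancelling of the current operation.
; Its construction script copies the user name from the game instance and assigns a widget class for each firefighter role, including the rescue dog.
; The CancelOperation input resets active operations such as move, chop, extinguish or carry to None.
; BeginPlay is empty, and a duplicate name-setting chain in the event graph never runs.
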(event EventBeginPlay)

(event Input|ActionEvents|InputActionCancelOperation
  (params (Key :type Key%20Structure))
  (:Pressed
    (bind _returnvalue (Class|FPPlayerController|GetCurrentOperation))
    (switch Utilities|FlowControl|Switch|SwitchonEGameOperations _returnvalue
      (:Move
        _)
      (:ChopWall
        _)
      (:ExtinguishFire
        _)
      (:Carry
        _)
      (:OpenDoor
        _)
      (:FireDeckGun
        _)
      (:FlipPOI
        _)
      (:Dodge
        _)
      (:Squeeze
        _))
    (Class|FPPlayerController|SetNone)))

(fn ConstructionScript
  (Utilities|FlowControl|Sequence
    (:then_0
      (bind _asbp_flash_point_game_instance (Utilities|Casting|CastToBP_FlashPointGameInstance (Game|GetGameInstance)))
      (Class|FPPlayerController|SetPlayerName (Utilities|String|ToString(Text) (Variables|/Game/BPs/GameMechanics/BP_FlashPointGameInstance.BP_FlashPointGameInstance_C|GetUserName _asbp_flash_point_game_instance))))
    (:then_1
      (Variables|Default|SetBasicFireFighterClass "/Game/BPs/Widgets/WBP_BasicFireFighter.WBP_BasicFireFighter_C"))
    (:then_2
      (Variables|Default|SetCAFSFireFighterClass "/Game/BPs/Widgets/WBP_CAFS_Firefighter.WBP_CAFS_Firefighter_C"))
    (:then_3
      (Variables|Default|SetDriverClass "/Game/BPs/Widgets/WBP_DriverOperator.WBP_DriverOperator_C"))
    (:then_4
      (Variables|Default|SetCaptainClass "/Game/BPs/Widgets/WBP_FireCaptain.WBP_FireCaptain_C"))
    (:then_5
      (Variables|Default|SetGeneralistClass "/Game/BPs/Widgets/WBP_Generalist.WBP_Generalist_C"))
    (:then_6
      (Variables|Default|SetHazTecClass "/Game/BPs/Widgets/WBP_HazmatTech.WBP_HazmatTech_C"))
    (:then_7
      (Variables|Default|SetImageTecClass "/Game/BPs/Widgets/WBP_ImagingTech.WBP_ImagingTech_C"))
    (:then_8
      (Variables|Default|SetParamedicClass "/Game/BPs/Widgets/WBP_Paramedic.WBP_Paramedic_C"))
    (:then_9
      (Variables|Default|SetRescueSpecClass "/Game/BPs/Widgets/WBP_RescueSpecialist.WBP_RescueSpecialist_C"))
    (:then_10
      (Variables|Default|SetRescueDogClass "/Game/BPs/Widgets/WBP_RescueDog.WBP_RescueDog_C"))
    (:then_11
      (Variables|Default|SetVeteranClass "/Game/BPs/Widgets/WBP_Veteran.WBP_Veteran_C"))))