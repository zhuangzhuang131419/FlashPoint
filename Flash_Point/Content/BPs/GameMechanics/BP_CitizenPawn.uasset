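; Citizen pawn that the player clicks to have it carried by a firefighter.
; Clicking its static mesh reads the current operation from FPPlayerController and calls AttachCitizenToFireFighter when that operation is Carry, with debug prints of the operation or a failed cast.
; The construction script calls SetMaterial on slot 0 of the FireFighter component without specifying a material.
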(event OnClicked(StaticMesh)
  (params (TouchedComponent :type Primitive%20Component%20Object%20Reference) (ButtonPressed :type Key%20Structure))
  (bind _asfpplayer_controller (Utilities|Casting|CastToFPPlayerController (Game|GetPlayerController 0))
    (:then
      (bind _returnvalue (Class|FPPlayerController|GetCurrentOperation _asfpplayer_controller))
      (Development|PrintString (Utilities|String|EnumtoString _returnvalue))
      (if (Utilities|Enum|Equal(Enum) _returnvalue "Carry")
        (Class|CitizenPawn|AttachCitizentoFireFighter)))
    (:CastFailed
      (Development|PrintString "Cast Failed"))))

(fn ConstructionScript
  (Rendering|Material|SetMaterial (Variables|Default|GetFireFighter) 0 0))