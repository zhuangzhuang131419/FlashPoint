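; BP_Door is a swinging door that starts blocked and opens when OnOpenDoor is triggered.
; OnOpenDoor marks it opened, clears the blocked flag and calls OpenDoor, which plays a timeline rotating the door 90 degrees in yaw from its frame's rotation.
; CloseDoor reverses the same timeline.
; A player controller cast on each timeline update has nothing wired after it.
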(event EventOpenDoor
  (bind _doorframe (Variables|Default|GetDoorFrame))
  (bind _relativerotation (Variables|/Script/Engine.SceneComponent|GetRelativeRotation _doorframe))
  (bind (_roll _pitch _yaw) (Math|Rotator|BreakRotator _relativerotation))
  ;[1 1 1] Open Door && Close Door
  (bind _newtrack_0 (Timeline|Timeline_2 Play)
    (:Update
      (Transformation|SetRelativeRotation (Variables|Default|GetDoor) (Math|Rotator|Lerp(Rotator) _relativerotation (Math|Rotator|MakeRotator _roll _pitch (+ _yaw 9e+01)) _newtrack_0) false false)
      (Utilities|Casting|CastToBP_FPPlayerController (Game|GetPlayerController 0)))))

(event EventOnOpenDoor
  ;[1 1 1] Initial open door on boundaries
  (Variables|Default|Setopened true)
  (Variables|Default|SetisBlocked false)
  (Class|Door|OpenDoor))

(event EventCloseDoor
  (bind _doorframe (Variables|Default|GetDoorFrame))
  (bind _relativerotation (Variables|/Script/Engine.SceneComponent|GetRelativeRotation _doorframe))
  (bind (_roll _pitch _yaw) (Math|Rotator|BreakRotator _relativerotation))
  ;[1 1 1] Open Door && Close Door
  (bind _newtrack_0 (Timeline|Timeline_2 Reverse)
    (:Update
      (Transformation|SetRelativeRotation (Variables|Default|GetDoor) (Math|Rotator|Lerp(Rotator) _relativerotation (Math|Rotator|MakeRotator _roll _pitch (+ _yaw 9e+01)) _newtrack_0) false false)
      (Utilities|Casting|CastToBP_FPPlayerController (Game|GetPlayerController 0)))))

(fn ConstructionScript
  (Variables|Default|SetisBlocked true))