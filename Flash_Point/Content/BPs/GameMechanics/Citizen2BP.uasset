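; Citizen2BP is a clickable citizen actor that can be brought to the player's position once.
; When its static mesh is clicked, it gets the current operation from FPPlayerController and prints it.
; If that operation is OpenDoor and NotWithPlayer is set, it moves itself to the player character's location without sweeping and clears the flag.
; It does not follow afterward, and the flag is only set again at BeginPlay.
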(event OnClicked(StaticMesh)
  (params (TouchedComponent :type Primitive%20Component%20Object%20Reference) (ButtonPressed :type Key%20Structure))
  (bind _asfpplayer_controller (Utilities|Casting|CastToFPPlayerController (Game|GetPlayerController 0))
    (:then
      (bind _returnvalue (Class|FPPlayerController|GetCurrentOperation _asfpplayer_controller))
      (Development|PrintString (Utilities|String|EnumtoString _returnvalue))
      (if (and (Utilities|Enum|Equal(Enum) _returnvalue "OpenDoor") (Variables|Default|GetNotWithPlayer))
        (Transformation|SetActorLocation (Transformation|GetActorLocation (Game|GetPlayerCharacter 0)) false false)
        (Variables|Default|SetNotWithPlayer false)))
    (:CastFailed
      (Development|PrintString "Cast Failed"))))

(event EventBeginPlay
  (Variables|Default|SetNotWithPlayer true))

(fn ConstructionScript)