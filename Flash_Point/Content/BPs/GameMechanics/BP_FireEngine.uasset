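; Fire engine Blueprint built around a mouse-positioned pop-up menu for getting in or out, leaving and firing the deck gun.
; BeginPlay caches the BP_FPPlayerController, creates WBP_FireEnginePopOut and binds its option events to handlers here.
; Only showing and removing the widget have bodies; the click and action events are empty.
; The logic that opens the menu on demand and drives the controller's fire engine states is disconnected and never runs.
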(event OnClicked(femesh)
  (params (TouchedComponent :type Primitive%20Component%20Object%20Reference) (ButtonPressed :type Key%20Structure)))

(event Custom|AddWidget
  (bind _returnvalue (Game|GetPlayerController 0))
  (bind _widgetpopup (Variables|Default|GetWidgetPopUp))
  (bind (_locationx _locationy) (Game|Player|GetMousePosition _returnvalue))
  (Class|UserWidget|SetPositioninViewport _widgetpopup (Math|Vector2D|MakeVector2D _locationx _locationy) true)
  (UserInterface|Viewport|AddtoViewport _widgetpopup 0)
  (Variables|Default|SetWidgetShowed true))

(event Custom|GetInCar)

(event Custom|LeaveFireEngine)

(event Custom|FireDeckGun)

(event Custom|RemoveWidget
  (Widget|RemovefromParent (Variables|Default|GetWidgetPopUp))
  (Variables|Default|SetWidgetShowed false))

(event Custom|GetOutFireEngine)

(event EventBeginPlay
  (bind _asbp_fpplayer_controller (Utilities|Casting|CastToBP_FPPlayerController (Game|GetPlayerController 0)))
  (Variables|Default|SetPlayerController _asbp_fpplayer_controller)
  (bind _returnvalue (UserInterface|CreateWidget "/Game/BPs/Widgets/WBP_FireEnginePopOut.WBP_FireEnginePopOut_C"))
  (bind _output_get (Variables|Default|SetWidgetPopUp _returnvalue))
  (EventDispatchers|BindEventtoOptionSelected _output_get (delegate Custom|RemoveWidget))
  (EventDispatchers|BindEventtoGetinFireEngineEvent _output_get (delegate Custom|GetInCar))
  (EventDispatchers|BindEventtoLeaveFireEngineEvent _output_get (delegate Custom|LeaveFireEngine))
  (EventDispatchers|BindEventtoFireDeckGunEvent _output_get (delegate Custom|FireDeckGun))
  (EventDispatchers|BindEventtoGetOutFireEngineEvent _output_get (delegate Custom|GetOutFireEngine)))

(fn ConstructionScript
  (Utilities|FlowControl|Sequence
    (:then_0
      (Variables|Default|SetfireEngineMesh 0))
    (:then_1
      (Variables|Default|SetFireEngineClass "/Game/BPs/Widgets/WBP_FireEnginePopOut.WBP_FireEnginePopOut_C"))))