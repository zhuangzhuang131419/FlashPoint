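; BP_SLGameBoard is a game board that generates its layout at play start and adds a keyboard-driven save/load of current game health.
; The construction script assigns tile, road, camera and POI classes, and BeginPlay calls GenerateSpecified with Indicator, then enables input for the FP player controller.
; N writes health into a MySaveGame slot, and M restores it from that slot if one exists and prints the value.
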(event EventBeginPlay
  (Utilities|FlowControl|Sequence
    (:then_0
      (Class|GameBoard|GenerateSpecified (Variables|Default|GetIndicator)))
    (:then_1
      (bind _asbp_fpplayer_controller (Utilities|Casting|CastToBP_FPPlayerController (Game|GetPlayerController 0)))
      (Input|EnableInput _asbp_fpplayer_controller))))

(event Input|KeyboardEvents|N
  (params (Key :type Key%20Structure))
  (:Pressed
    (bind _returnvalue (SaveGame|CreateSaveGameObject "/Game/_PersonalFolder/Cheng/MySaveGame.MySaveGame_C"))
    (bind _output_get (Variables|Default|SetSaverSubClass _returnvalue))
    (bind _asmy_save_game (Utilities|Casting|CastToMySaveGame _output_get))
    (bind _returnvalue_2 (Class|GameBoard|GetCurrentGameHealth))
    (Variables|/Game/_PersonalFolder/Cheng/MySaveGame.MySaveGame_C|SetHealth _asmy_save_game _returnvalue_2)
    (SaveGame|SaveGametoSlot (Variables|Default|GetSaverSubClass) (Variables|Default|GetSaveSlot1))))

(event Input|KeyboardEvents|M
  (params (Key :type Key%20Structure))
  (:Pressed
    (bind _returnvalue (SaveGame|DoesSaveGameExist (Variables|Default|GetSaveSlot1)))
    (if _returnvalue
      (bind _returnvalue_2 (SaveGame|LoadGamefromSlot (Variables|Default|GetSaveSlot1)))
      (bind _asmy_save_game (Utilities|Casting|CastToMySaveGame _returnvalue_2))
      (Class|GameBoard|SetCurrentGameHealth (Variables|/Game/_PersonalFolder/Cheng/MySaveGame.MySaveGame_C|GetHealth _asmy_save_game))
      (Development|PrintString (Utilities|String|ToString(Integer) (Variables|/Game/_PersonalFolder/Cheng/MySaveGame.MySaveGame_C|GetHealth _asmy_save_game))))))

(fn ConstructionScript
  (Utilities|FlowControl|Sequence
    (:then_0
      (Variables|Default|SetTileClass "/Game/BPs/GameMechanics/BP_Tile.BP_Tile_C"))
    (:then_1
      (Variables|Default|SetRoadClass "/Game/BPs/GameMechanics/BP_Road.BP_Road_C"))
    (:then_2
      (Variables|Default|SetCameraClass "/Game/BPs/GameMechanics/IndividualCamera.IndividualCamera_C"))
    (:then_3
      (Variables|Default|SetPOIClass "/Game/BPs/GameMechanics/BP_POI.BP_POI_C"))))