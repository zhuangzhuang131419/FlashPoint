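; BP_Door is a clickable door that swings open and closed when the player controller is in OpenDoor operation mode.
; Clicks on the wall mesh, frame or door share one handler, which flips IsOpen and plays or reverses a timeline.
; Timeline updates lerp the door's relative yaw between the frame's rotation and 90 degrees beyond it, calling SetNone on BP_FPPlayerController each update.
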(event OnClicked(WallMesh)
  (params (TouchedComponent :type Primitive%20Component%20Object%20Reference) (ButtonPressed :type Key%20Structure))
  (bind _doorframe (Variables|Default|GetDoorFrame))
  (bind _relativerotation (Variables|/Script/Engine.SceneComponent|GetRelativeRotation _doorframe))
  (bind (_roll _pitch _yaw) (Math|Rotator|BreakRotator _relativerotation))
  ;[1 1 1] Click open and close door
  (bind _asbp_fpplayer_controller (Utilities|Casting|CastToBP_FPPlayerController (Game|GetPlayerController 0)))
  (bind _returnvalue (Class|FPPlayerController|GetCurrentOperation _asbp_fpplayer_controller))
  (if (Utilities|Enum|Equal(Enum) _returnvalue "OpenDoor")
    (if (Variables|Default|GetisOpen)
      (Variables|Default|SetisOpen false)
      (bind _newtrack_0 (Timeline|Timeline_0 Reverse)
        (:Update
          (Transformation|SetRelativeRotation (Variables|Default|GetDoor) (Math|Rotator|Lerp(Rotator) _relativerotation (Math|Rotator|MakeRotator _roll _pitch (+ _yaw 9e+01)) _newtrack_0) false false)
          (Class|FPPlayerController|SetNone _asbp_fpplayer_controller)))
      (else
        (Variables|Default|SetisOpen true)
        (Timeline|Timeline_0 Play)))))

(event OnClicked(DoorFrame)
  (params (TouchedComponent :type Primitive%20Component%20Object%20Reference) (ButtonPressed :type Key%20Structure))
  (bind _doorframe (Variables|Default|GetDoorFrame))
  (bind _relativerotation (Variables|/Script/Engine.SceneComponent|GetRelativeRotation _doorframe))
  (bind (_roll _pitch _yaw) (Math|Rotator|BreakRotator _relativerotation))
  ;[1 1 1] Click open and close door
  (bind _asbp_fpplayer_controller (Utilities|Casting|CastToBP_FPPlayerController (Game|GetPlayerController 0)))
  (bind _returnvalue (Class|FPPlayerController|GetCurrentOperation _asbp_fpplayer_controller))
  (if (Utilities|Enum|Equal(Enum) _returnvalue "OpenDoor")
    (if (Variables|Default|GetisOpen)
      (Variables|Default|SetisOpen false)
      (bind _newtrack_0 (Timeline|Timeline_0 Reverse)
        (:Update
          (Transformation|SetRelativeRotation (Variables|Default|GetDoor) (Math|Rotator|Lerp(Rotator) _relativerotation (Math|Rotator|MakeRotator _roll _pitch (+ _yaw 9e+01)) _newtrack_0) false false)
          (Class|FPPlayerController|SetNone _asbp_fpplayer_controller)))
      (else
        (Variables|Default|SetisOpen true)
        (Timeline|Timeline_0 Play)))))

(event OnClicked(Door)
  (params (TouchedComponent :type Primitive%20Component%20Object%20Reference) (ButtonPressed :type Key%20Structure))
  (bind _doorframe (Variables|Default|GetDoorFrame))
  (bind _relativerotation (Variables|/Script/Engine.SceneComponent|GetRelativeRotation _doorframe))
  (bind (_roll _pitch _yaw) (Math|Rotator|BreakRotator _relativerotation))
  ;[1 1 1] Click open and close door
  (bind _asbp_fpplayer_controller (Utilities|Casting|CastToBP_FPPlayerController (Game|GetPlayerController 0)))
  (bind _returnvalue (Class|FPPlayerController|GetCurrentOperation _asbp_fpplayer_controller))
  (if (Utilities|Enum|Equal(Enum) _returnvalue "OpenDoor")
    (if (Variables|Default|GetisOpen)
      (Variables|Default|SetisOpen false)
      (bind _newtrack_0 (Timeline|Timeline_0 Reverse)
        (:Update
          (Transformation|SetRelativeRotation (Variables|Default|GetDoor) (Math|Rotator|Lerp(Rotator) _relativerotation (Math|Rotator|MakeRotator _roll _pitch (+ _yaw 9e+01)) _newtrack_0) false false)
          (Class|FPPlayerController|SetNone _asbp_fpplayer_controller)))
      (else
        (Variables|Default|SetisOpen true)
        (Timeline|Timeline_0 Play)))))

(event EventBeginPlay)

(event Collision|EventActorBeginOverlap
  (params (OtherActor :type Actor%20Object%20Reference)))

(event EventTick
  (params (DeltaSeconds :type Float%20%28single-precision%29)))

(fn ConstructionScript)