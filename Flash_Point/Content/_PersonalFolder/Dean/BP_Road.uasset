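; BP_Road is a road Blueprint that supplies materials and related classes, apparently for a grid-based board with movement and vehicle parking.
; Its Construction Script assigns materials for hidden, move-able, move-unable, engine and ambulance parking, and odd/even quadrant looks.
; It also sets the edge, wall and door class references to their Blueprint versions.
; The Event Graph holds only disabled default events, so none of the logic using these values is in these graphs.
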(event EventBeginPlay)

(event Collision|EventActorBeginOverlap
  (params (OtherActor :type Actor%20Object%20Reference)))

(event EventTick
  (params (DeltaSeconds :type Float%20%28single-precision%29)))

(fn ConstructionScript
  (Utilities|FlowControl|Sequence
    (:then_0
      (Utilities|FlowControl|Sequence
        (:then_0
          (Variables|Default|SethiddenMat "/Game/_PersonalFolder/Dean/HiddenMat.HiddenMat"))
        (:then_1
          (Variables|Default|SetableMat "/Game/_PersonalFolder/Dean/MoveAble.MoveAble"))
        (:then_2
          (Variables|Default|SetunableMat "/Game/_PersonalFolder/Dean/MoveUnable.MoveUnable"))
        (:then_3
          (Variables|Default|SetengineParkMat "/Game/_PersonalFolder/Dean/EngineParkMat.EngineParkMat"))
        (:then_4
          (Variables|Default|SetambulanceParkMat "/Game/_PersonalFolder/Dean/AmbulanceParkMat.AmbulanceParkMat"))
        (:then_5
          (Variables|Default|SetoddMat "/Game/_PersonalFolder/Dean/OddQuadrantMat.OddQuadrantMat"))
        (:then_6
          (Variables|Default|SetevenMat "/Game/_PersonalFolder/Dean/EvenQuadrantMat.EvenQuadrantMat"))))
    (:then_1
      (Utilities|FlowControl|Sequence
        (:then_0
          (Variables|Default|SetEdgeClass "/Game/_PersonalFolder/Dean/BP_Edge.BP_Edge_C"))
        (:then_1
          (Variables|Default|SetWallClass "/Game/BPs/GameMechanics/BP_Wall.BP_Wall_C"))
        (:then_2
          (Variables|Default|SetDoorClass "/Game/_PersonalFolder/Dean/BP_Door.BP_Door_C"))))))